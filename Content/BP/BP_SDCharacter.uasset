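; BP_SDCharacter is a character Blueprint that handles player movement, look and jump through Enhanced Input.
; Move and look actions pass their values to Move and Look functions defined outside this graph, while jump calls Jump on start and StopJumping on completion.
; Tick prints the gravity scale of SDCharacterMovementComponent to the screen every frame as a debug readout.
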(event `self.ReceiveTick`
  (params (DeltaSeconds :type "Float (single-precision)"))
  (`KismetSystemLibrary.PrintString` (`KismetStringLibrary.Conv_DoubleToString` (`CharacterMovementComponent.GravityScale` (`self.SDCharacterMovementComponent`))) true true (struct :`G` 0.66 :`B` 1.0 :`A` 1.0) 0.01))

(event `EnhancedInput|/Game/BP/Input/IA_Move`
  (params (ActionValue :type "Vector2D Structure") (ElapsedSeconds :type "Float (double-precision)") (TriggeredSeconds :type "Float (double-precision)") (InputAction :type "InputAction Object Reference" :default "/Game/BP/Input/IA_Move.IA_Move"))
  ;[1 1 1] Input
  (:`Triggered`
    (`self.Move` ActionValue)))

(event `EnhancedInput|/Game/BP/Input/IA_Look`
  (params (ActionValue :type "Vector2D Structure") (ElapsedSeconds :type "Float (double-precision)") (TriggeredSeconds :type "Float (double-precision)") (InputAction :type "InputAction Object Reference" :default "/Game/BP/Input/IA_Look.IA_Look"))
  ;[1 1 1] Input
  (:`Triggered`
    (`self.Look` ActionValue)))

(event `EnhancedInput|/Game/BP/Input/IA_Jump`
  (params (ActionValue :type Boolean) (ElapsedSeconds :type "Float (double-precision)") (TriggeredSeconds :type "Float (double-precision)") (InputAction :type "InputAction Object Reference" :default "/Game/BP/Input/IA_Jump.IA_Jump"))
  ;[1 1 1] Input
  (:`Started`
    (`self.Jump`))
  (:`Completed`
    (`self.StopJumping`)))

(fn `UserConstructionScript`)